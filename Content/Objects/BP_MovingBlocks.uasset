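; BP_MovingBlocks is an actor with two block components, LeftSide and RightSide, that slide back and forth in opposite directions along their relative X axis.
; MoveLeft and MoveRight offset the current relative X by MoveDist while keeping rotation.
; From BeginPlay, a Sequence runs paired one-second MoveComponentTo moves on both sides in parallel.
; Only the LeftSide chain calls MoveBlocks again, restarting the cycle for both.
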(event `self.ReceiveBeginPlay`
  (`self.MoveBlocks`))

(event `MoveBlocks`
  (`|ExecutionSequence`
    (:`then_0`
      (bind (_newposition _newrotation) (`self.MoveLeft` (`self.LeftSide`)))
      (`KismetSystemLibrary.MoveComponentTo` (`self.LeftSide`) _newposition _newrotation false false 1.0)
      (bind (_newposition_2 _newrotation_2) (`self.MoveRight` (`self.LeftSide`)))
      (`KismetSystemLibrary.MoveComponentTo` (`self.LeftSide`) _newposition_2 _newrotation_2 false false 1.0)
      (`self.MoveBlocks`))
    (:`then_1`
      (bind (_newposition_3 _newrotation_3) (`self.MoveRight` (`self.RightSide`)))
      (`KismetSystemLibrary.MoveComponentTo` (`self.RightSide`) _newposition_3 _newrotation_3 false false 1.0)
      (bind (_newposition_4 _newrotation_4) (`self.MoveLeft` (`self.RightSide`)))
      (`KismetSystemLibrary.MoveComponentTo` (`self.RightSide`) _newposition_4 _newrotation_4 false false 1.0))))

(fn `MoveLeft`
  (params (Mesh :type "StaticMeshComponent Object Reference"))
  (returns (NewPosition :type "Vector Structure") (NewRotation :type "Rotator Structure"))
  (bind (_relativelocation_x _relativelocation_y _relativelocation_z) (`KismetMathLibrary.BreakVector` (`SceneComponent.RelativeLocation` Mesh)))
  (return (`KismetMathLibrary.MakeVector` (- _relativelocation_x (`self.MoveDist`)) _relativelocation_y _relativelocation_z) (`SceneComponent.RelativeRotation` Mesh)))

(fn `MoveRight`
  (params (Mesh :type "StaticMeshComponent Object Reference"))
  (returns (NewPosition :type "Vector Structure") (NewRotation :type "Rotator Structure"))
  (bind (_relativelocation_x _relativelocation_y _relativelocation_z) (`KismetMathLibrary.BreakVector` (`SceneComponent.RelativeLocation` Mesh)))
  (return (`KismetMathLibrary.MakeVector` (+ _relativelocation_x (`self.MoveDist`)) _relativelocation_y _relativelocation_z) (`SceneComponent.RelativeRotation` Mesh)))

(fn `UserConstructionScript`)